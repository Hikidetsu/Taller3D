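; BP_Puerta is a door Blueprint that slides its Cube component upward when the OpenDoor event is called.
; BeginPlay caches the cube's starting relative location.
; OpenDoor plays Timeline_SubirPuerta from the start, using its Alpha to lerp the cube from that location to OpenHeight above it, without sweeping.
; It has no closing logic, and nothing in the Blueprint itself calls OpenDoor.
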(event Custom|Open%20Door
  (bind _initiallocation (Variables|Default|GetInitialLocation))
  (bind (_x _y _z) (Math|Vector|BreakVector _initiallocation))
  (bind _alpha (Timeline|Timeline_SubirPuerta PlayFromStart)
    (:Update
      (Transformation|SetRelativeLocation (Variables|Default|GetCube) (Math|Vector|Lerp(Vector) (Variables|Default|GetInitialLocation) (Math|Vector|MakeVector _x _y (+ _z (Variables|Default|GetOpenHeight))) _alpha) false false))))

(event EventBeginPlay
  (Variables|Default|SetInitialLocation (Variables|/Script/Engine.SceneComponent|GetRelativeLocation (Variables|Default|GetCube))))

(event Collision|EventActorBeginOverlap
  (params (OtherActor :type Actor%20Object%20Reference)))

(event EventTick
  (params (DeltaSeconds :type Float%20%28single-precision%29)))

(fn ConstructionScript)